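; BP_SH_Matter_Child is a child projectile whose one-shot ability creates a zero-gravity force burst around its small, scaled-down sphere.
; UseAbility activates the radial force, swaps the sphere's material and runs a zero-length multi-sphere trace as an area query.
; Physics-simulating components it hits lose gravity, with no restore here, and have their names printed for debugging.
; After a short delay it calls ChangeCamera.
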(event `self.UseAbility`
  (bind _sphere (`self.Sphere`))
  (bind _returnvalue (`SceneComponent.K2_GetComponentLocation` _sphere))
  (`/Engine/EditorBlueprintResources/StandardMacros.DoOnce` false
    (:`Completed`
      (`ActorComponent.SetActive` (`self.RadialForce`) true false)
      (`PrimitiveComponent.SetMaterial` _sphere 0 "/Engine/BufferVisualization/Anisotropy.Anisotropy")
      (bind _outhits (`KismetSystemLibrary.SphereTraceMulti` _returnvalue _returnvalue 400.0 "TraceTypeQuery1"))
      (for _array_element _outhits
        (bind (_bblockinghit _binitialoverlap _time _distance _location _impactpoint _normal _impactnormal _physmat _hitactor _hitcomponent) (`GameplayStatics.BreakHitResult` _array_element))
        (if (`SceneComponent.IsSimulatingPhysics` _hitcomponent "None")
          (`PrimitiveComponent.SetEnableGravity` _hitcomponent false)
          (`KismetSystemLibrary.PrintString` (`KismetSystemLibrary.GetDisplayName` _hitcomponent))))
      (`KismetSystemLibrary.Delay` 3.0)
      (`self.ChangeCamera`))))

(fn `UserConstructionScript`
  (`parent.UserConstructionScript`)
  (`SceneComponent.SetWorldScale3D` (`self.Sphere`) (0.4 0.4 0.4)))