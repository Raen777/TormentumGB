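; Child projectile Blueprint that splits into three smaller balls when its ability is used or it hits anything other than BP_PawnThrower.
; UseAbility runs once, spawning half-scale BP_MiniBall_Child actors at increasing Y and Z offsets from the sphere.
; Each keeps the sphere's X and Z physics velocity with a fixed negative Y speed.
; The projectile then calls a camera change and destroys itself.
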(event `self.UseAbility`
  (bind _sphere (`self.Sphere`))
  (bind (_velocity_x _velocity_y _velocity_z) (`KismetMathLibrary.BreakVector` (`self.Velocity`)))
  (bind (_returnvalue_x _returnvalue_y _returnvalue_z) (`KismetMathLibrary.BreakVector` (`SceneComponent.K2_GetComponentLocation` _sphere)))
  (bind (_returnvalue_x_2 _returnvalue_y_2 _returnvalue_z_2) (`KismetMathLibrary.BreakVector` (+ (`KismetMathLibrary.MakeVector` 0.0 _returnvalue_y _returnvalue_z) (`self.Coef_Loc`))))
  (`/Engine/EditorBlueprintResources/StandardMacros.DoOnce` false
    (:`Completed`
      (bind _returnvalue (`PrimitiveComponent.GetPhysicsLinearVelocity` _sphere "None"))
      (set `self.Velocity` _returnvalue)
      (for _ (range 3)
        (set `self.Coef_Loc` (+ (`self.Coef_Loc`) 50.0))
        (bind _returnvalue_2 (`|SpawnActorFromClass` "/Game/MyGame/Blueprints/Projectiles/BP_MiniBall_Child.BP_MiniBall_Child_C" (`KismetMathLibrary.MakeTransform` (`KismetMathLibrary.MakeVector` _returnvalue_x _returnvalue_y_2 _returnvalue_z_2) (struct) (0.5 0.5 0.5)) "AlwaysSpawn" "OverrideRootScale" null null))
        (`PrimitiveComponent.SetPhysicsLinearVelocity` (`/Game/MyGame/Blueprints/Projectiles/BP_ThrownPawn.Sphere` _returnvalue_2) (`KismetMathLibrary.MakeVector` _velocity_x -1000.0 _velocity_z) false "None"))
      (`self.ChangeCamera`)
      (`self.K2_DestroyActor`))))

(event `self.ReceiveHit`
  (params (MyComp :type "PrimitiveComponent Object Reference") (Other :type "Actor Object Reference") (OtherComp :type "PrimitiveComponent Object Reference") (bSelfMoved :type Boolean) (HitLocation :type "Vector Structure") (HitNormal :type "Vector Structure") (NormalImpulse :type "Vector Structure") (Hit :type "HitResult Structure (by ref)"))
  (cast `/Game/MyGame/Blueprints/Environment/BP_PawnThrower` Other
    (:`CastFailed`
      (`self.UseAbility`))))

(fn `UserConstructionScript`
  (`parent.UserConstructionScript`))