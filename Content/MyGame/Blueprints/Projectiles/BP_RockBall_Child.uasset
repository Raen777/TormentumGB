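; Child rock ball projectile Blueprint that supplies its own one-shot ability.
; UseAbility passes through a DoOnce, launches the Sphere upward with a velocity-change impulse, then calls ChangeCamera after a short delay.
; No reset is wired to the DoOnce, and the construction script just runs the parent's.
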(event `self.UseAbility`
  (`/Engine/EditorBlueprintResources/StandardMacros.DoOnce` false
    (:`Completed`
      (`PrimitiveComponent.AddImpulse` (`self.Sphere`) (0.0 0.0 800.0) "None" true)
      (`KismetSystemLibrary.Delay` 3.0)
      (`self.ChangeCamera`))))

(fn `UserConstructionScript`
  (`parent.UserConstructionScript`))