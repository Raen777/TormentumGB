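; BP_Bomb_Child is a bomb projectile variant that explodes when its UseAbility event fires.
; A DoOnce guards the explosion, which applies radial damage with falloff from the sphere's location, ignoring the bomb itself, and fires a radial force impulse.
; It then calls for a camera change and destroys itself.
; The construction script runs the parent's setup and shrinks the sphere, and BeginPlay defers to the parent.
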(event `self.ReceiveBeginPlay`
  (`parent.ReceiveBeginPlay`))

(event `self.UseAbility`
  (`/Engine/EditorBlueprintResources/StandardMacros.DoOnce` false
    (:`Completed`
      (`GameplayStatics.ApplyRadialDamageWithFalloff` 80.0 10.0 (`SceneComponent.K2_GetComponentLocation` (`self.Sphere`)) 200.0 250.0 0.5 null (`|MakeArray` self :!type "Actor Object Reference") self null)
      (`RadialForceComponent.FireImpulse` (`self.RadialForce`))
      (`self.ChangeCamera`)
      (`self.K2_DestroyActor`))))

(fn `UserConstructionScript`
  (`parent.UserConstructionScript`)
  (`SceneComponent.SetWorldScale3D` (`self.Sphere`) (0.8 0.8 0.8)))