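; BP_TNT_Box_Child is an explosive TNT box, a child Blueprint that blasts its surroundings when destroyed.
; On Destroyed, it applies radial damage with distance falloff from the Mesh location, then fires the RadialForce impulse.
; The construction script only calls the parent, and BeginPlay, overlap and Tick are disabled stubs.
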(event `self.ReceiveDestroyed`
  (`GameplayStatics.ApplyRadialDamageWithFalloff` :`BaseDamage` 100.0 :`MinimumDamage` 10.0 :`Origin` (`SceneComponent.K2_GetComponentLocation` (`self.Mesh`)) :`DamageInnerRadius` 250.0 :`DamageOuterRadius` 500.0 :`DamageCauser` self :`InstigatedByController` null)
  (`RadialForceComponent.FireImpulse` (`self.RadialForce`)))

(fn `UserConstructionScript`
  (`parent.UserConstructionScript`))