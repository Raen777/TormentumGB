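; Destructible plane prop that loses HP from physics hits and radial damage, then spawns an effect and adds its kill score to the game mode when destroyed.
; After a one-second immortality window at BeginPlay, hits passing a positive Y/Z velocity threshold deal damage scaled by impulse.
; Those hits also start a one-second timer that enables mesh gravity.
; Zero HP triggers a retriggerable delay before destruction.
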(event `self.ReceiveBeginPlay`
  (bind _asbp_my_game_mode (cast `/Game/MyGame/Blueprints/BP_MyGameMode` (`GameplayStatics.GetGameMode`)))
  (set `self.As My Game Mode` _asbp_my_game_mode)
  (`KismetSystemLibrary.Delay` 1.0)
  (set `self.Immortality?` false))

(event `self.Mesh.OnComponentHit`
  (params (HitComponent :type "PrimitiveComponent Object Reference") (OtherActor :type "Actor Object Reference") (OtherComp :type "PrimitiveComponent Object Reference") (NormalImpulse :type "Vector Structure") (Hit :type "HitResult Structure (by ref)"))
  (if (not (`self.Immortality?`))
    (bind _dodamage_ (`self.CheckVelocityFunc` HitComponent 3.0))
    (if _dodamage_
      (bind _output_get (set `self.HP_Decrease` (/ (`KismetMathLibrary.VSize` NormalImpulse) 1000.0)))
      (`self.DecreaseHP`)
      (`KismetSystemLibrary.K2_SetTimerDelegate` (delegate `CustomEvent_0`) 1.0)
      (`KismetSystemLibrary.PrintString` (`KismetStringLibrary.Concat_StrStr` "HIT by " (`KismetStringLibrary.Conv_DoubleToString` _output_get)) true true (struct :`R` 1.0 :`B` 0.007908 :`A` 1.0)))))

(event `CustomEvent_0`
  (`PrimitiveComponent.SetEnableGravity` (`self.Mesh`) true))

(event `DecreaseHP`
  ;[1 1 1] HP decrease and destroy actor
  (bind _output_get (set `self.HP` (- (`self.HP`) (`self.HP_Decrease`))))
  (if (<= _output_get 0.0)
    (`KismetSystemLibrary.RetriggerableDelay` (`self.DestroyDelay`))
    (`GameplayStatics.SpawnEmitterAtLocation` (`self.EmitterDestroy`) (`SceneComponent.K2_GetComponentLocation` (`self.Mesh`)))
    (`self.K2_DestroyActor`)))

(event `self.ReceiveDestroyed`
  (bind _as_my_game_mode (`self.As My Game Mode`))
  ;[1 1 1] send score to game mode
  (set `/Game/MyGame/Blueprints/BP_MyGameMode.Com_Score` (+ (`/Game/MyGame/Blueprints/BP_MyGameMode.Com_Score` _as_my_game_mode) (`self.KillScore`)) _as_my_game_mode))

(event `self.ReceiveRadialDamage`
  (params (DamageReceived :type "Float (single-precision)") (DamageType :type "DamageType Object Reference") (Origin :type "Vector Structure") (HitInfo :type "HitResult Structure (by ref)") (InstigatedBy :type "Controller Object Reference") (DamageCauser :type "Actor Object Reference"))
  (set `self.HP_Decrease` DamageReceived)
  (`self.DecreaseHP`))

(fn `CheckVelocityFunc`
  (params (Target :type "PrimitiveComponent Object Reference") (MinVelocity :type "Float (double-precision)"))
  (returns (`DoDamage?` :type Boolean))
  (locals (M_Vel :type "Float (double-precision)" :default 3.0))
  (set `local.M_Vel` MinVelocity)
  (bind _returnvalue (`PrimitiveComponent.GetPhysicsLinearVelocity` Target "None"))
  (bind _returnvalue_2 (`PrimitiveComponent.GetPhysicsLinearVelocity` (`self.Mesh`) "None"))
  (return (or (or (>= (.y _returnvalue_2) (`local.M_Vel`)) (>= (.z _returnvalue_2) (`local.M_Vel`))) (or (>= (.y _returnvalue) (`local.M_Vel`)) (>= (.z _returnvalue) (`local.M_Vel`))))))

(fn `UserConstructionScript`)