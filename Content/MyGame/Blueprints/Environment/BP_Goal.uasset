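; BP_Goal is a goal actor placed in the environment whose destruction feeds the game's win check.
; On Destroyed it runs the parent logic, then passes itself to CheckWinFunc on the game mode reference.
; GetScoreFunc returns its input score unchanged, while BeginPlay and the construction script only call their parents.
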(event `self.ReceiveBeginPlay`
  (`parent.ReceiveBeginPlay`))

(event `self.ReceiveDestroyed`
  (`parent.ReceiveDestroyed`)
  (`/Game/MyGame/Blueprints/BP_MyGameMode.CheckWinFunc` (`self.As My Game Mode`) self))

(fn `GetScoreFunc`
  (params (InScore :type Integer :default 0))
  (returns (OutScore :type Integer))
  (return InScore))

(fn `UserConstructionScript`
  (`parent.UserConstructionScript`))