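; BP_MyHUD is a Blueprint that manages the game's start screen and main UI.
; On BeginPlay it creates and shows the Widget_GameStart_Over screen with UI-only input focused on it, and pre-creates Widget_Main without displaying it.
; It binds to the start widget's AddWidgetToViewport dispatcher, which adds the main widget to the viewport and switches input to Game and UI.
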(event `self.ReceiveBeginPlay`
  (bind _returnvalue (`GameplayStatics.GetPlayerController` 0))
  (`/Engine/EditorBlueprintResources/StandardMacros.IsValid` (`self.WidgetGameStartRef`)
    (:`Is Valid`
      _)
    (:`Is Not Valid`
      (bind _returnvalue_2 (`|CreateWidget` "/Game/MyGame/UI/Widget_GameStart_Over.Widget_GameStart_Over_C" _returnvalue))
      (bind _output_get (set `self.WidgetGameStartRef` _returnvalue_2))))
  (`WidgetBlueprintLibrary.SetInputMode_UIOnlyEx` _returnvalue _output_get)
  (`UserWidget.AddToViewport` _output_get 0)
  (`/Engine/EditorBlueprintResources/StandardMacros.IsValid` (`self.WidgetMainRef`)
    (:`Is Valid`
      _)
    (:`Is Not Valid`
      (bind _returnvalue_3 (`|CreateWidget` "/Game/MyGame/UI/Widget_Main.Widget_Main_C" (`GameplayStatics.GetPlayerController` 0)))
      (set `self.WidgetMainRef` _returnvalue_3)))
  (add `/Game/MyGame/UI/Widget_GameStart_Over.AddWidgetToViewport` _output_get (delegate `AddWidgetToViewport_Event_0`)))

(event `AddWidgetToViewport_Event_0`
  (`UserWidget.AddToViewport` (`self.WidgetMainRef`) 0)
  (`WidgetBlueprintLibrary.SetInputMode_GameAndUIEx` (`GameplayStatics.GetPlayerController` 0) null "DoNotLock" false))

(fn `UserConstructionScript`)