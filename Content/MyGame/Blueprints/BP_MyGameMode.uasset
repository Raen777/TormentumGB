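; Game mode that handles level progression, goal-based win checks and the unlocked-level list.
; BeginPlay loads level index and score from BP_GameInstance's save and gathers all BP_Goal actors.
; SetupLvlFunc builds level names from an enum and fills a combo box up to the given index.
; CheckWinFunc removes goals, saves progress once none remain, and opens the next level, or the IndexLvl level when projectiles run out.
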(event `self.ReceiveBeginPlay`
  (bind _asbp_game_instance (cast `/Game/MyGame/Blueprints/BP_GameInstance` (`GameplayStatics.GetGameInstance`)))
  (bind _output_get (set `self.As BP Game Instance` _asbp_game_instance))
  (bind (_outputindex _outputscore) (`/Game/MyGame/Blueprints/BP_GameInstance.GetVarInSaveFunc` _output_get))
  (set `self.IndexLvl` _outputindex)
  (set `self.Com_Score` _outputscore)
  (bind _outactors (`GameplayStatics.GetAllActorsOfClass` "/Game/MyGame/Blueprints/Environment/BP_Goal.BP_Goal_C"))
  (set `self.Out Actors` _outactors))

(fn `CheckWinFunc`
  (params (InActor :type "/Game/MyGame/Blueprints/Environment/BP_Goal Object Reference"))
  (bind _out_actors (`self.Out Actors`))
  (bind _lvlnames_array (`self.LvlNames_array`))
  (bind _returnvalue (<= (`self.Com_Proj_Count`) 0))
  (`/Engine/EditorBlueprintResources/StandardMacros.IsValid` InActor
    (:`Is Valid`
      (`KismetArrayLibrary.Array_RemoveItem` _out_actors InActor))
    (:`Is Not Valid`
      _))
  (if (== (`KismetArrayLibrary.Array_Length` _out_actors) 0)
    (bind _returnvalue_2 (`GameplayStatics.GetCurrentLevelName` true))
    (bind _result (`/Engine/EditorBlueprintResources/StandardMacros.IncrementInt` (`KismetArrayLibrary.Array_Find` _lvlnames_array _returnvalue_2))
      (:`  `
        (`/Game/MyGame/Blueprints/BP_GameInstance.SetVarInSaveFunc` (`self.As BP Game Instance`) (`self.Com_Score`) _result)
        (`GameplayStatics.OpenLevel` (select `bool` _returnvalue :`false` (`KismetStringLibrary.Conv_StringToName` (`|GetArrayItem` _lvlnames_array _result)) :`true` (`KismetStringLibrary.Conv_StringToName` (`|GetArrayItem` (`self.LvlNames_array`) (`self.IndexLvl`)))) :!label _label)
        (`KismetSystemLibrary.PrintString` (`KismetStringLibrary.Conv_IntToString` (`self.IndexLvl`)) true true (struct :`G` 0.370833 :`B` 0.046658 :`A` 1.0))))
    (elif _returnvalue
      (goto _label))))

(fn `SetupLvlFunc`
  (params (IndexLvl :type Integer) (ComboBoxRef :type "ComboBoxString Object Reference"))
  (bind _lvlnames_array (`self.LvlNames_array`))
  (bind _output_get (set `self.IndexLvl` IndexLvl))
  (`KismetArrayLibrary.Array_Clear` _lvlnames_array)
  (bind _enumvalue (foreach `/Game/MyGame/Blueprints/LevelsNames_Enum` false)
    (:`LoopBody`
      (`KismetArrayLibrary.Array_AddUnique` (`self.LvlNames_array`) (`|GetEnumeratorNameAsString` _enumvalue)))
    (:`then`
      (for _index (range (+ (`KismetMathLibrary.Clamp` _output_get 0 (`KismetArrayLibrary.Array_LastIndex` _lvlnames_array)) 1))
        (`ComboBoxString.AddOption` ComboBoxRef (`|GetArrayItem` _lvlnames_array _index))))))

(fn `UserConstructionScript`)